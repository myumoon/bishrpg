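; Test character Blueprint that displays a modular character built from Accessory, Hair, Face, Upper and Lower skeletal meshes.
; SetCharacterId builds per-part asset paths from an ID and looks them up through the Asset Registry into mesh variables.
; The construction script applies those variables to the mesh components, with Lower on the main Mesh.
; Its ID check includes a constant-false comparison, so it never calls SetCharacterId.
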(event `self.ReceiveBeginPlay`
  (`parent.ReceiveBeginPlay`))

(fn `ApplySkeletalMesh`
  (`SkinnedMeshComponent.SetSkinnedAssetAndUpdate` (`self.FacePartsMesh`) (`self.Accessory`) true)
  (`SkinnedMeshComponent.SetSkinnedAssetAndUpdate` (`self.HairMesh`) (`self.Hair`) true)
  (`SkinnedMeshComponent.SetSkinnedAssetAndUpdate` (`self.FaceMesh`) (`self.Face`) true)
  (`SkinnedMeshComponent.SetSkinnedAssetAndUpdate` (`self.UpperMesh`) (`self.Upper`) true)
  (`SkinnedMeshComponent.SetSkinnedAssetAndUpdate` (`self.Mesh`) (`self.Lower`) true))

(fn `GetSkeletalMeshAsset`
  (params (AssetPath :type String) (SetTo :type "SkeletalMesh Object Reference (by ref)"))
  (returns (SetSkeletalMesh :type "SkeletalMesh Object Reference"))
  (bind _returnvalue (message `AssetRegistry.GetAssetByObjectPath` (`KismetSystemLibrary.Conv_InterfaceToObject` (`AssetRegistryHelpers.GetAssetRegistry`)) (`KismetStringLibrary.Conv_StringToName` AssetPath) true))
  (bind _asskeletal_mesh (cast `SkeletalMesh` (`AssetRegistryHelpers.GetAsset` _returnvalue))
    (:`then`
      (`|VariableSetRef` SetTo _asskeletal_mesh))
    (:`CastFailed`
      (`|VariableSetRef` SetTo _asskeletal_mesh)))
  (return _asskeletal_mesh))

(fn `Is Valid Character Id`
  (returns (Valid :type Boolean))
  (return (and (`KismetStringLibrary.NotEqual_StrStr` (`self.CharacterId`)) (> 0 0))))

(fn `MakeCostumeAssetPath`
  (params (CharacterId :type String))
  (returns (AccessoryPath :type String) (HairPath :type String) (FacePath :type String) (UpperPath :type String) (LowerPath :type String))
  (return (`self.MakeCostumeAssetPathWithParts` "Accessory" CharacterId) (`self.MakeCostumeAssetPathWithParts` "Hair" CharacterId) (`self.MakeCostumeAssetPathWithParts` "Face" CharacterId) (`self.MakeCostumeAssetPathWithParts` "Upper" CharacterId) (`self.MakeCostumeAssetPathWithParts` "Lower" CharacterId)))

(fn `MakeCostumeAssetPathWithParts`
  (params (Parts :type String) (InString :type String))
  (returns (AssetPath :type String))
  (return (`KismetTextLibrary.Conv_TextToString` (`|FormatText` "/Game/Characters/Parts/{parts}/Meshes/Parts{parts}_{id}.Parts{parts}_{id}" (`KismetTextLibrary.Conv_StringToText` Parts) (`KismetTextLibrary.Conv_StringToText` InString)))))

(fn `SetCharacterId`
  (params (CharacterId :type String))
  (bind (_accessorypath _hairpath _facepath _upperpath _lowerpath) (`self.MakeCostumeAssetPath` CharacterId))
  (`self.GetSkeletalMeshAsset` _accessorypath (`self.Accessory`))
  (`self.GetSkeletalMeshAsset` _hairpath (`self.Hair`))
  (`self.GetSkeletalMeshAsset` _facepath (`self.Face`))
  (`self.GetSkeletalMeshAsset` _upperpath (`self.Upper`))
  (`self.GetSkeletalMeshAsset` _lowerpath (`self.Lower`)))

(fn `UserConstructionScript`
  (`parent.UserConstructionScript`)
  (`|ExecutionSequence`
    (:`then_0`
      (if (`self.Is Valid Character Id`)
        (`self.SetCharacterId` (`self.CharacterId`))))
    (:`then_1`
      (`self.ApplySkeletalMesh`))))