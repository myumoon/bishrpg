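; Normal enemy character that takes damage when hit and, on defeat, turns into the Seisouin model and releases a player soul actor.
; Capsule overlaps on a custom collision channel flag the hit animation, spawn a fire impact and reduce HP.
; At zero HP it swaps meshes, plays stand-up, disables capsule collision and runs a timeline driving the appear-rate parameter on Seisouin's dynamic materials, created at BeginPlay.
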(event `self.ReceiveBeginPlay`
  (`parent.ReceiveBeginPlay`)
  (`|ExecutionSequence`
    (:`then_0`
      (`self.CreateDynamicMaterialInstance` 0 (`self.SeisouinMaterial`) 500.0 -140.0))
    (:`then_1`
      (`self.CreateDynamicMaterialInstance` 1 (`self.SeisouinMaterial`) 500.0 -140.0))
    (:`then_2`
      (`self.CreateDynamicMaterialInstance` 2 (`self.SeisouinMaterial`) 500.0 -140.0))))

(event `self.CapsuleComponent.OnComponentBeginOverlap`
  (params (OverlappedComponent :type "PrimitiveComponent Object Reference") (OtherActor :type "Actor Object Reference") (OtherComp :type "PrimitiveComponent Object Reference") (OtherBodyIndex :type Integer) (bFromSweep :type Boolean) (SweepResult :type "HitResult Structure (by ref)"))
  (bind _seisouin (`self.Seisouin`))
  (if (`|EnumEquality` (`PrimitiveComponent.GetCollisionObjectType` OtherComp) "ECC_GameTraceChannel1")
    (bind _ascharacter_anim_bp (cast `/Game/Characters/Animations/CharacterAnimBP` (`SkeletalMeshComponent.GetAnimInstance` (`self.Mesh`))))
    (set `/Game/Characters/Animations/CharacterAnimBP.IsHit` true _ascharacter_anim_bp)
    (`GameplayStatics.SpawnEmitterAtLocation` "/Game/InfinityBladeEffects/Effects/FX_Mobile/Impacts/P_Impact_Player_Fire_Medium.P_Impact_Player_Fire_Medium" (`SceneComponent.K2_GetComponentLocation` OtherComp))
    (bind _output_get (set `self.HP` (- (`self.HP`) 40)))
    (if (<= _output_get 0)
      (`/Engine/EditorBlueprintResources/StandardMacros.DoOnce` false
        (:`Completed`
          (`|ExecutionSequence`
            (:`then_0`
              (`SceneComponent.SetVisibility` (`self.Mesh`) false false)
              (`SceneComponent.SetVisibility` _seisouin true false)
              (bind _ascharacter_anim_bp_2 (cast `/Game/Characters/Animations/CharacterAnimBP` (`SkeletalMeshComponent.GetAnimInstance` _seisouin)))
              (set `/Game/Characters/Animations/CharacterAnimBP.IsStandup` true _ascharacter_anim_bp_2)
              (`PrimitiveComponent.SetCollisionEnabled` (`self.CapsuleComponent`) "NoCollision"))
            (:`then_1`
              (`|SpawnActorFromClass` "/Game/Particles/P_PlayerSoul_BP.P_PlayerSoul_BP_C" (`self.GetTransform`) "AlwaysSpawn" "OverrideRootScale" null null))
            (:`then_2`
              (bind (_direction _alpha) (`Timeline|ModelFadeTimeline` :!via `PlayFromStart`)
                (:`Update`
                  (for _array_element (`self.SeisouinMaterial`)
                    (`MaterialInstanceDynamic.SetScalarParameterValue` _array_element "AppearRateParam" _alpha)))))))))))

(fn `CreateDynamicMaterialInstance`
  (params (MatIndex :type Integer) (MatAry :type "Array of MaterialInstanceDynamic Object Reference") (MaxAppearHeight :type "Float (double-precision)") (HeightOffset :type "Float (double-precision)"))
  (returns (Seisouin :type "MaterialInstanceDynamic Object Reference"))
  (bind _returnvalue (`PrimitiveComponent.CreateDynamicMaterialInstance` (`self.Seisouin`) MatIndex "/Game/Characters/Materials/OthersCommonMat.OthersCommonMat"))
  (`KismetArrayLibrary.Array_Add` MatAry _returnvalue)
  (`MaterialInstanceDynamic.SetScalarParameterValue` _returnvalue "MaxAppearHeightParam" MaxAppearHeight)
  (`MaterialInstanceDynamic.SetScalarParameterValue` _returnvalue "BaseHeightOffsetParam" HeightOffset)
  (return _returnvalue))

(fn `UserConstructionScript`
  (`parent.UserConstructionScript`))