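; BP_IceFallProjectile is a projectile actor for an ice-fall battle effect that bursts on its first overlap.
; When its sphere begins an overlap, it deactivates the projectile effect, disables collision and activates the ice hit effect at the sweep location.
; It also shakes the camera, stops projectile movement and removes the point light, then destroys itself after a delay.
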(event `self.Sphere_0.OnComponentBeginOverlap`
  (params (OverlappedComponent :type "PrimitiveComponent Object Reference") (OtherActor :type "Actor Object Reference") (OtherComp :type "PrimitiveComponent Object Reference") (OtherBodyIndex :type Integer) (bFromSweep :type Boolean) (SweepResult :type "HitResult Structure (by ref)"))
  (bind _hiteffectice (`self.HitEffectIce`))
  (`|ExecutionSequence`
    (:`then_0`
      (`ActorComponent.Deactivate` (`self.Projectile`))
      (`PrimitiveComponent.SetCollisionEnabled` (`self.Sphere_0`) "NoCollision")
      (`ActorComponent.SetActive` _hiteffectice true false)
      (`SceneComponent.K2_SetWorldLocation` _hiteffectice (`.Location` (`GameplayStatics.BreakHitResult` SweepResult)) false false)
      (`/Game/NkLib/NkUtil.ShakeCamera` "/Game/Battle/Camera/DamegeCameraShake_Normal.DamegeCameraShake_Normal_C")
      (`ActorComponent.SetActive` (`self.ProjectileMovement`) false false)
      (`ActorComponent.K2_DestroyComponent` (`self.PointLight`)))
    (:`then_2`
      (`KismetSystemLibrary.Delay` 5.0)
      (`self.K2_DestroyActor`))))

(fn `UserConstructionScript`)