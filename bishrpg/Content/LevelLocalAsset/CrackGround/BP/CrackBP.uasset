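; Crack-ground actor that lays out a voxel crack along an editable spline, built entirely in the Construction Script.
; CalcBlockPlacementsWithArea turns the route spline, start/end widths, sampling interval and offset into block placements in a voxel block context.
; Placements passing IsSetHole become crack wall instanced meshes at block centers, then the crack is debug-drawn.
; Refresh resets on each construction; the line-based placement variant is left disconnected.
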(fn `UserConstructionScript`
  (set `self.Refresh` false)
  (bind _results (`VoxelCrackHelper.CalcBlockPlacementsWithArea` (`self.VoxelBlockContext`) (`self.CrackRouteSpline`) (`self.StartWidth`) (`self.EndWidth`) (`self.SplineSeparateLength`) (`self.SetOffset`)))
  (for _array_element _results
    (if (`VoxelCrackHelper.IsSetHole` _array_element)
      (`InstancedStaticMeshComponent.AddInstanceWorldSpace` (`self.CrackWallInstancedStaticMesh`) (`KismetMathLibrary.MakeTransform` (`.CenterPos` (break `VoxelBlockInfo` _array_element))))))
  (`VoxelCrackHelper.DebugDrawVoxelCrack` self (`self.VoxelBlockContext`) (struct :`R` 0.171797 :`G` 0.532203 :`B` 1.0 :`A` 1.0) 50.0 2.0))