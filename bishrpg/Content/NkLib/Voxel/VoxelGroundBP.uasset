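; Voxel ground actor for painting and erasing grid-snapped blocks on an InstancedStaticMesh, with saving of changes.
; Insert toggles editing with its menu and debug camera; a held press line-traces under the cursor, removing any block in each newly entered cell and adding one in Brush mode.
; A Morton-indexed QuadTreeIndex maps positions to instance indices for lookup.
; Removal moves the last instance into the freed slot to keep indices stable.
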(event `self.ReceiveBeginPlay`
  (`self.SetupUI`)
  (`self.RegisterMeshToQuadTree`))

(event `OnReset`
  (`InstancedStaticMeshComponent.ClearInstances` (`self.InstancedStaticMesh`))
  (`QuadTreeIndexComponent.ClearAll` (`self.QuadTreeIndex`)))

(event `OnSave`
  (`EditorExtensionFunctionLibrary.SaveSimulationChanges` self))

(event `Key|Insert` :consume false
  (params (Key :type "Key Structure"))
  (:`Pressed`
    (`self.ToggleEditMode`)))

(event `InputTouch` :consume false
  (params (Location :type "Vector Structure") (FingerIndex :type "ETouchIndex Enum"))
  (:`Pressed`
    (set `self.MousePressed` true))
  (:`Released`
    (set `self.MousePressed` false)))

(event `self.ReceiveTick`
  (params (DeltaSeconds :type "Float (single-precision)"))
  (if (`self.EditEnabled`)
    ;[1 1 1] 編集
    (bind (_fixedpos _movable) (`self.UpdateMouse`))
    (if _movable
      (bind (_mortonindex _array_element) (`self.ForeachMortonIndex` _fixedpos :!label _label)
        (:`LoopBody`
          (bind (_returnvalue _location) (`self.GetInstanceLocation` _array_element))
          (if _returnvalue
            (if (<= (`KismetMathLibrary.VSizeSquared` (- _location _fixedpos)) 10.0)
              (`self.RemoveInstance` _array_element _mortonindex)
              (`self.SetInstanceCountToUI`)
              (goto _label :!via `Break`))))
        (:`Completed`
          (switch `/Game/NkLib/Voxel/VoxelEditMode` (`self.EditMode`)
            (:`NewEnumerator0`
              (`self.AddInstance` _fixedpos)
              (`self.SetInstanceCountToUI`))))))))

(fn `AddInstance`
  (params (Pos :type "Vector Structure"))
  (bind _returnvalue (`InstancedStaticMeshComponent.AddInstanceWorldSpace` (`self.InstancedStaticMesh`) (`KismetMathLibrary.MakeTransform` Pos)))
  (`QuadTreeIndexComponent.Add` (`self.QuadTreeIndex`) Pos _returnvalue))

(fn `FixMousePosition`
  (params (Pos :type "Vector Structure"))
  (returns (FixedPos :type "Vector Structure"))
  (bind _blockinterval (`self.BlockInterval`))
  (return (`KismetMathLibrary.MakeVector` (* (`KismetMathLibrary.FFloor` (+ (.x (/ Pos (`self.BlockInterval`))) 0.5)) _blockinterval) (* (`KismetMathLibrary.FFloor` (+ (.y (/ Pos (`self.BlockInterval`))) 0.5)) _blockinterval) (* (`KismetMathLibrary.FFloor` (.z (/ Pos (`self.BlockInterval`)))) _blockinterval))))

(fn `GetInstanceLocation`
  (params (InstanceIndex :type Integer))
  (returns (ReturnValue :type Boolean) (Location :type "Vector Structure"))
  (bind (_outinstancetransform _returnvalue) (`InstancedStaticMeshComponent.GetInstanceTransform` (`self.InstancedStaticMesh`) InstanceIndex true))
  (return _returnvalue (.location _outinstancetransform)))

(fn `IsMovedCell`
  (params (Pos :type "Vector Structure"))
  (returns (CanMove :type Boolean))
  (return (!= Pos (`self.PrevSelectedPos`))))

(fn `IsNearPosition`)

(fn `RegisterMeshToQuadTree`
  (for _index (range (`InstancedStaticMeshComponent.GetInstanceCount` (`self.InstancedStaticMesh`)))
    (bind (_mortonindex _returnvalue) (`QuadTreeIndexComponent.Add` (`self.QuadTreeIndex`) (.location (`InstancedStaticMeshComponent.GetInstanceTransform` (`self.InstancedStaticMesh`) _index true)) _index))))

(fn `RemoveInstance`
  (params (InstanceIndex :type Integer) (targetMortonIndex :type "MortonIndex Structure (by ref)"))
  (returns (Removed :type Boolean))
  ;[1 1 1] 位置をずらして最高インデックスを削除
  (bind _returnvalue (`QuadTreeIndexComponent.Remove` (`self.QuadTreeIndex`) InstanceIndex targetMortonIndex)) ; まずは削除対象の領域を消す
  (`QuadTreeIndexComponent.Replace` (`self.QuadTreeIndex`) (- (`InstancedStaticMeshComponent.GetInstanceCount` (`self.InstancedStaticMesh`)) 1) InstanceIndex true) ; 最高要素のインデックスを削除対象のインデックスに差し替えて再利用
  (`self.ReplaceRemoveInstance` InstanceIndex) ; 削除インデックスのメッシュ位置を最高要素のメッシュ位置に移動
  (`|ExecutionSequence`
    (:`then_1`
      (return _returnvalue))))

(fn `ReplaceRemoveInstance`
  (params (Index :type Integer))
  (bind _instancedstaticmesh (`self.InstancedStaticMesh`))
  (bind _returnvalue (- (`InstancedStaticMeshComponent.GetInstanceCount` _instancedstaticmesh) 1))
  (`InstancedStaticMeshComponent.UpdateInstanceTransform` _instancedstaticmesh Index (`InstancedStaticMeshComponent.GetInstanceTransform` _instancedstaticmesh _returnvalue true) true true true)
  (`InstancedStaticMeshComponent.RemoveInstance` _instancedstaticmesh _returnvalue))

(fn `SetEditMode`
  (params (EditMode :type "/Game/NkLib/Voxel/VoxelEditMode Enum" :default "NewEnumerator0"))
  (set `self.EditMode` EditMode))

(fn `SetInstanceCountToUI`
  (`/Game/NkLib/Voxel/UI/VoxelGroundMenu.SetBoxCount` (`self.Menu`) (`InstancedStaticMeshComponent.GetInstanceCount` (`self.InstancedStaticMesh`))))

(fn `SetupUI`
  (bind _returnvalue (`|CreateWidget` "/Game/NkLib/Voxel/UI/VoxelGroundMenu.VoxelGroundMenu_C"))
  (set `self.Menu` _returnvalue)
  (`UserWidget.AddToViewport` _returnvalue 0)
  (`Widget.SetVisibility` _returnvalue "Hidden")
  (`/Game/NkLib/Voxel/UI/VoxelGroundMenu.Initialize` _returnvalue self))

(fn `ToggleEditMode`
  (bind _camera (`/Game/NkLib/Debug/Camera/NkDebugCameraUtil.FindDebugCamera`))
  (bind _output_get (set `self.EditEnabled` (not (`self.EditEnabled`))))
  (if _output_get
    (`Widget.SetVisibility` (`self.Menu`) "Visible")
    (`/Engine/EditorBlueprintResources/StandardMacros.IsValid` _camera
      (:`Is Valid`
        (`/Game/NkLib/Debug/Camera/NkDebugCamera.Enable` _camera)))
    (else
      (`Widget.SetVisibility` (`self.Menu`) "Hidden")
      (`/Engine/EditorBlueprintResources/StandardMacros.IsValid` _camera
        (:`Is Valid`
          (`/Game/NkLib/Debug/Camera/NkDebugCamera.Disable` _camera))))))

(fn `UpdateMouse`
  (returns (FixedPos :type "Vector Structure") (Movable :type Boolean))
  (bind (_worldlocation _worlddirection _returnvalue) (`PlayerController.DeprojectMousePositionToWorld` (`GameplayStatics.GetPlayerController` 0)))
  (if (`self.MousePressed`)
    (if _returnvalue
      (bind (_outhit _returnvalue_2) (`KismetSystemLibrary.LineTraceSingleForObjects` :`Start` _worldlocation :`End` (+ _worldlocation (* _worlddirection 10000.0)) :`ObjectTypes` (`|MakeArray` "ObjectTypeQuery1" :!type "EObjectTypeQuery Enum") :`DrawDebugType` "ForOneFrame"))
      (if _returnvalue_2
        (bind _fixedpos (`self.FixMousePosition` (`.Location` (`GameplayStatics.BreakHitResult` _outhit))))
        (bind _movable (`self.UpdateMovable` _fixedpos)))
      (return _fixedpos _movable))))

(fn `UpdateMovable`
  (params (Pos :type "Vector Structure"))
  (returns (Movable :type Boolean))
  (locals (CanMove :type Boolean))
  (bind _output_get (set `local.CanMove` (`self.IsMovedCell` Pos)))
  (if _output_get
    (set `self.PrevSelectedPos` Pos))
  (return _output_get))

(fn `UserConstructionScript`
  (`QuadTreeIndexComponent.DebugDrawAtConstructionScript` (`self.QuadTreeIndex`) (struct :`R` 0.367334 :`G` 0.887153 :`B` 0.678057 :`A` 1.0) 5.0))