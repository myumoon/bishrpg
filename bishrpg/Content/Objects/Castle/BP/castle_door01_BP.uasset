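; Castle double door that swings open when anything begins overlapping its OpenBox trigger, with no actor filter or closing logic.
; The Open event scales a timeline's play rate to the requested duration and plays it from the start, interpolating from OpenAngle to the target angle.
; UpdateDoorAngle mirrors the yaw across both leaves, and the construction script uses it to pose them at OpenAngle.
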(event `Open`
  (params (Angle :type "Float (double-precision)") (Time :type "Float (double-precision)"))
  (`TimelineComponent.SetPlayRate` (`self.OpenDoorTimeline`) (/ 1.0 Time))
  (bind (_direction _rate) (`Timeline|OpenDoorTimeline` :!via `PlayFromStart`)
    (:`Update`
      (`self.UpdateDoorAngle` (`KismetMathLibrary.Lerp` (`self.OpenAngle`) Angle _rate)))))

(event `self.OpenBox.OnComponentBeginOverlap`
  (params (OverlappedComponent :type "PrimitiveComponent Object Reference") (OtherActor :type "Actor Object Reference") (OtherComp :type "PrimitiveComponent Object Reference") (OtherBodyIndex :type Integer) (bFromSweep :type Boolean) (SweepResult :type "HitResult Structure (by ref)"))
  (`self.Open` 120.0 2.0))

(fn `UpdateDoorAngle`
  (params (Angle :type "Float (double-precision)"))
  (`SceneComponent.K2_SetRelativeRotation` (`self.DoorL`) (`KismetMathLibrary.MakeRotator` 0.0 0.0 (- 360.0 Angle)) false false)
  (`SceneComponent.K2_SetRelativeRotation` (`self.DoorR`) (`KismetMathLibrary.MakeRotator` 0.0 0.0 Angle) false false))

(fn `UserConstructionScript`
  (`self.UpdateDoorAngle` (`self.OpenAngle`)))