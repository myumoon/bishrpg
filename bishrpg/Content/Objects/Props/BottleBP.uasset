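; Bottle prop that fakes liquid inside it through a dynamic material instance on its "Inner" material slot.
; Each tick sets the water surface offset from fill rate and bounds, blending per-axis heights by the bottle's tilt against world up.
; A cyclic position history yields a movement strength that drives wave height and interval, stepped multiplicatively toward their targets and clamped.
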(event `self.ReceiveBeginPlay`)

(event `self.ReceiveTick`
  (params (DeltaSeconds :type "Float (single-precision)"))
  (`self.UpdateWaveHeight`)
  (`self.UpdateWaterHeight`))

(fn `AddPosHistory`
  (params (Pos :type "Vector Structure"))
  (bind _oldvalue (`/Game/NkLib/Maxros/NkMacro.IncrementCycle` (`self.PosAddIndex`) (`self.MaxPosHistory`))
    (:`Exit`
      (`KismetArrayLibrary.Array_Set` (`self.PosHistory`) _oldvalue Pos true))))

(fn `CalcCurrentWaterHeight`
  (returns (Height :type "Float (double-precision)"))
  (bind _returnvalue (`KismetMathLibrary.Vector_Up`))
  (bind (_x _y _z) (`KismetMathLibrary.GetAxes` (`self.K2_GetActorRotation`)))
  (bind _returnvalue_2 (* (`KismetMathLibrary.GetPI`) 0.5))
  (bind _returnvalue_3 (+ (- 1.0 (/ (`/Game/NkLib/NkUtil.CalcAngleRad` _returnvalue (`KismetMathLibrary.Vector_GetAbs` _y) true) _returnvalue_2)) 1e-06))
  (bind _returnvalue_4 (+ (- 1.0 (/ (`/Game/NkLib/NkUtil.CalcAngleRad` _returnvalue (`KismetMathLibrary.Vector_GetAbs` _z) true) _returnvalue_2)) 1e-05))
  (bind _returnvalue_5 (`KismetMathLibrary.Lerp` (.x (`self.GetWaterHeight`)) (.y (`self.GetWaterHeight`)) (- 1.0 (`KismetMathLibrary.FClamp` (/ (+ (- 1.0 (/ (`/Game/NkLib/NkUtil.CalcAngleRad` _returnvalue (`KismetMathLibrary.Vector_GetAbs` _x) true) _returnvalue_2)) _returnvalue_3) _returnvalue_3)))))
  (return (`KismetMathLibrary.Lerp` _returnvalue_5 (.z (`self.GetWaterHeight`)) (- 1.0 (`KismetMathLibrary.FClamp` (/ (+ _returnvalue_5 _returnvalue_4) _returnvalue_4))))))

(fn `CalcMoveDeltaAverage`
  (returns (Average :type "Vector Structure"))
  (locals (Sum :type "Vector Structure"))
  (bind _poshistory (`self.PosHistory`))
  (bind _poshistory_2 (`self.PosHistory`))
  (for _index (range 1 (`KismetArrayLibrary.Array_Length` _poshistory_2))
    (set `local.Sum` (+ (`local.Sum`) (- (`|GetArrayItem` _poshistory _index) (`|GetArrayItem` _poshistory (- _index 1))))))
  (return (/ (`local.Sum`) (`KismetArrayLibrary.Array_Length` _poshistory_2))))

(fn `CalcStrengthRate`
  (returns (Rate :type "Float (double-precision)"))
  (bind _average (`self.CalcMoveDeltaAverage`))
  (return (`KismetMathLibrary.FClamp` (/ (`KismetMathLibrary.VSize` _average) (`self.MaxWaveThreshold`)))))

(fn `Get Wave Height`
  (params (StrengthRate :type "Float (double-precision)"))
  (returns (Height :type "Float (double-precision)"))
  (return (`KismetMathLibrary.Lerp` (`self.MinWaveHeight`) (`self.MaxWaveHeight`) StrengthRate)))

(fn `GetInterp`
  (params (Current :type "Float (double-precision)") (Prev :type "Float (double-precision)") (UpRate :type "Float (double-precision)" :default 1.5) (DownRate :type "Float (double-precision)" :default 0.95))
  (returns (ReturnValue :type "Float (double-precision)"))
  (return (`KismetMathLibrary.SelectFloat` (* Prev UpRate) (* Prev DownRate) (>= Current Prev))))

(fn `GetWaterHeight`
  (returns (HeightBounds :type "Vector Structure"))
  (return (* (* (`self.WaterBoundsSize`) 0.5) (* (- (`self.WaterRate`) 0.5) 2.0))))

(fn `GetWaveInterval`
  (params (StrengthRate :type "Float (double-precision)"))
  (returns (Interval :type "Float (double-precision)"))
  (return (`KismetMathLibrary.Lerp` (`self.MinWaveInterval`) (`self.MaxWaveInterval`) StrengthRate)))

(fn `SetMaterial`
  (bind _bottle (`self.Bottle`))
  (bind _returnvalue (`MeshComponent.GetMaterialIndex` _bottle "Inner"))
  (bind _returnvalue_2 (`PrimitiveComponent.CreateDynamicMaterialInstance` (`self.Bottle`) _returnvalue (`PrimitiveComponent.GetMaterial` _bottle _returnvalue) "InnerMat"))
  (set `self.InnerMat` _returnvalue_2))

(fn `UpdateWaterHeight`
  (bind _height (`self.CalcCurrentWaterHeight`))
  (`MaterialInstanceDynamic.SetScalarParameterValue` (`self.InnerMat`) "WaterSurfaceOffset" _height))

(fn `UpdateWaveHeight`
  (`self.AddPosHistory` (`self.K2_GetActorLocation`))
  (bind _rate (`self.CalcStrengthRate`))
  (bind _output_get (set `self.PrevWaveHeight` (`KismetMathLibrary.FClamp` (`self.GetInterp` (`self.Get Wave Height` _rate) (`self.PrevWaveHeight`)) (`self.MinWaveHeight`) (`self.MaxWaveHeight`))))
  (bind _output_get_2 (set `self.PrevWaveInterval` (`KismetMathLibrary.FClamp` (`self.GetInterp` (`self.GetWaveInterval` _rate) (`self.PrevWaveInterval`) 1.03 0.9) (`self.MaxWaveInterval`) (`self.MinWaveInterval`))))
  (`MaterialInstanceDynamic.SetScalarParameterValue` (`self.InnerMat`) "WaveHeightX" _output_get)
  (`MaterialInstanceDynamic.SetScalarParameterValue` (`self.InnerMat`) "WaveHeightY" (+ _output_get 0.5))
  (`MaterialInstanceDynamic.SetScalarParameterValue` (`self.InnerMat`) "WaveIntervalX" _output_get_2)
  (`MaterialInstanceDynamic.SetScalarParameterValue` (`self.InnerMat`) "WaveIntervalY" (+ _output_get_2 0.1)))

(fn `UserConstructionScript`
  (`self.SetMaterial`)
  (`self.UpdateWaterHeight`))